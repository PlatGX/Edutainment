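; Demonstration bike that animates rotational motion for numbered modes 2.4, 2.5.1 and 2.5.2, covering angular acceleration and change of rotational axis.
; A wheel timeline spins the front wheel and polls for mode changes, launching each mode's sequence.
; Sequences toggle omega/alpha arrows and use fixed delays to advance from 2.5.1 to 2.5.2 and start the fork rotation.
; Play-rate lerping and arrow spawning have no callers here; several functions are stubs.
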(event `self.ReceiveBeginPlay`
  (bind _bikemode (`self.BikeMode`))
  (`self.RotateWheel`)
  (switch `/Game/BikeAnim/E_BikeMode` _bikemode
    (:`NewEnumerator0`
      (set `self.NewEnum` _bikemode)
      (set `self.Velocity` 2.0)
      (set `self.Acceleration` 0.0))
    (:`NewEnumerator1`
      (set `self.NewEnum` _bikemode)
      (`self.AngularAccelerationSequence`))
    (:`NewEnumerator2`
      (set `self.NewEnum` _bikemode)
      (`self.ChangeOfRotationalAxisSequence`))))

(event `RotateWheel`
  (bind _fwheel (`self.FWheel`))
  (bind _newenum (`self.NewEnum`))
  (bind (_returnvalue_roll _returnvalue_pitch _returnvalue_yaw) (`KismetMathLibrary.BreakRotator` (`SceneComponent.K2_GetComponentRotation` _fwheel)))
  ; Currently 2π rad/s, 1 rev/s, or 360°/s.
  ;; For example, if Play Rate is set to .5, all above will be halved.
  (bind (_direction _wheelrotation) (`Timeline|T_Wheel`)
    (:`Update`
      (`SceneComponent.K2_SetWorldRotation` _fwheel (`KismetMathLibrary.MakeRotator` _wheelrotation _returnvalue_pitch _returnvalue_yaw) false false)
      (if (not (`|EnumEquality` (`self.BikeMode`) _newenum))
        (bind _output_get (set `self.BikeMode` _newenum))
        (switch `/Game/BikeAnim/E_BikeMode` _output_get
          (:`NewEnumerator0`
            (set `self.Velocity` 2.0)
            (set `self.Acceleration` 0.0))
          (:`NewEnumerator1`
            (`self.HideRotationAxisArrows`)
            (`self.AngularAccelerationSequence`))
          (:`NewEnumerator2`
            (`self.HideAccelerationArrows`)
            (`self.ChangeOfRotationalAxisSequence`)))))))

(event `CreateArrowSpawner`
  ; Misc. Junk, potentially good reference
  (bind _returnvalue (`|SpawnActorFromClass` "/Game/Blueprints/ArrowTest/ProceduralArrowTest/BP_SpawnProceduralArrows.BP_SpawnProceduralArrows_C" (`self.GetTransform`) "Undefined" "MultiplyWithRoot" null null))
  (set `self.ArrowSpawner` _returnvalue))

(event `CalculatePlayRate`
  (params (PlayRate :type "Float (double-precision)"))
  ; Misc. Junk, potentially good reference
)

(event `AngularAccelerationSequence`
  (bind _output_get (set `self.Velocity` 1.0))
  (set `self.Acceleration` 0.0)
  (`TimelineComponent.SetPlayRate` (`self.T_Wheel`) _output_get)
  (`self.ShowAccelerationArrows`)
  (`KismetSystemLibrary.Delay` 108.0)
  (set `self.NewEnum` "NewEnumerator2"))

(event `ShowAccelerationArrows`
  (`SceneComponent.SetVisibility` (`self.OmegaArrow`) true true)
  (`SceneComponent.SetVisibility` (`self.AlphaArrow`) true true))

(event `HideAccelerationArrows`
  (`SceneComponent.SetVisibility` (`self.OmegaArrow`) false true)
  (`SceneComponent.SetVisibility` (`self.AlphaArrow`) false true))

(event `LerpPlayRate`
  (params (LerpStart :type "Float (double-precision)") (LerpEnd :type "Float (double-precision)"))
  (bind (_direction _acceleration) (`Timeline|T_AccelerationLerp`)
    (:`Update`
      (bind _output_get (set `self.PlayRate` (`KismetMathLibrary.Lerp` LerpStart LerpEnd _acceleration)))
      (`TimelineComponent.SetPlayRate` (`self.T_Wheel`) _output_get))))

(event `RotateFork`
  (bind (_direction _handlerotation) (`Timeline|T_ForkRotation`)
    (:`Update`
      (if (> _handlerotation (`self.CurValue`))
        (`SceneComponent.K2_AddLocalRotation` (`self.ForkAndBar`) (`KismetMathLibrary.MakeRotator` 0.0 0.0 1.0) false false)
        (else
          (`SceneComponent.K2_AddLocalRotation` (`self.ForkAndBar`) (`KismetMathLibrary.MakeRotator` 0.0 0.0 -1.0) false false)))
      (set `self.CurValue` _handlerotation))))

(event `ChangeOfRotationalAxisSequence`
  (set `self.Velocity` 1.0)
  (set `self.Acceleration` 0.0)
  (`self.ShowRotationAxisArrows`)
  (`KismetSystemLibrary.Delay` 18.0)
  (`self.RotateFork`))

(event `ShowRotationAxisArrows`
  (`SceneComponent.SetVisibility` (`self.Omega21Arrow`) true true)
  (`SceneComponent.SetVisibility` (`self.Omega1Arrow`) true true)
  (`SceneComponent.SetVisibility` (`self.Omega2Arrow`) true true)
  (`SceneComponent.SetVisibility` (`self.Alpha2Arrow`) true true))

(event `HideRotationAxisArrows`
  (`SceneComponent.SetVisibility` (`self.Omega21Arrow`) false true)
  (`SceneComponent.SetVisibility` (`self.Omega1Arrow`) false true)
  (`SceneComponent.SetVisibility` (`self.Omega2Arrow`) false true)
  (`SceneComponent.SetVisibility` (`self.Alpha2Arrow`) false true))

(fn `SetAcceleration`)

(fn `SetVelocity`)

(fn `UpdateSpeed`
  (params (TimelineFloat :type "Float (double-precision)"))
  (returns (NewFloat :type "Float (double-precision)"))
  (return (* TimelineFloat (`self.Acceleration`))))

(fn `UserConstructionScript`)