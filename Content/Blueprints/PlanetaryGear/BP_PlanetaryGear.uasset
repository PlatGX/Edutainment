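; Planetary gear set actor that plays looping clockwise or counter-clockwise animations and highlights the planet, sun or ring gears.
; Tick polls boolean flags to play or stop the animation and to update materials.
; DoOnce gates keep the animation from restarting every frame, and stopping resets both.
; While material focus is enabled, each gear's material slot swaps between normal and focus materials according to its own flag.
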(event `Ring Gear`
  ; Ring Gear
  (`PrimitiveComponent.SetMaterial` (`self.planetary_gears`) 3 "/Game/Blueprints/PlanetaryGear/Materials/MI_RingGearFocus.MI_RingGearFocus"))

(event `Sun Gear`
  ; Sun Gear
  (`PrimitiveComponent.SetMaterial` (`self.planetary_gears`) 1 "/Game/Blueprints/PlanetaryGear/Materials/MI_SunGearFocus.MI_SunGearFocus"))

(event `Material Focus`
  ; Material Hierarchy
  (if (`self.bAreWeFocusingMaterial?`)
    (`|ExecutionSequence`
      (:`then_0`
        (if (`self.bFocusPlanetGear`)
          (`self.Planet Gear`)
          (else
            (`PrimitiveComponent.SetMaterial` (`self.planetary_gears`) 0 "/Game/Blueprints/PlanetaryGear/Materials/MI_PlanetGear.MI_PlanetGear"))))
      (:`then_1`
        (if (`self.bFocusSunGear`)
          (`self.Sun Gear`)
          (else
            (`PrimitiveComponent.SetMaterial` (`self.planetary_gears`) 1 "/Game/Blueprints/PlanetaryGear/Materials/MI_SunGear.MI_SunGear"))))
      (:`then_2`
        (if (`self.bFocusRingGear`)
          (`self.Ring Gear`)
          (else
            (`PrimitiveComponent.SetMaterial` (`self.planetary_gears`) 3 "/Game/Blueprints/PlanetaryGear/Materials/MI_RingGear.MI_RingGear")))))))

(event `Planet Gear`
  ; Planet Gear
  (`PrimitiveComponent.SetMaterial` (`self.planetary_gears`) 0 "/Game/Blueprints/PlanetaryGear/Materials/MI_PlanetGearFocus.MI_PlanetGearFocus"))

(event `self.ReceiveTick`
  (params (DeltaSeconds :type "Float (single-precision)"))
  ; Planetary Hierarchy
  (`|ExecutionSequence`
    (:`then_0`
      (if (`self.bIsAnimationplaying?`)
        (if (`self.bAnimationClockwise?`)
          (`self.Animation Clockwise`)
          (else
            (`self.Animation CounterClockwise`)))
        (else
          (`self.Stop Animation`))))
    (:`then_1`
      (`self.Material Focus`))))

(event `Stop Animation`
  (`SkeletalMeshComponent.Stop` (`self.planetary_gears`))
  (`self.Reset Do Once`))

(event `Animation Clockwise`
  (bind _planetary_gears (`self.planetary_gears`))
  ; Planetary Gear Animation (Clockwise / Counter Clockwise)
  (`/Engine/EditorBlueprintResources/StandardMacros.DoOnce` false :!label _label
    (:`Completed`
      (`SkeletalMeshComponent.PlayAnimation` _planetary_gears "/Game/Blueprints/PlanetaryGear/SkeletalMeshes/planetary_gears_Anim.planetary_gears_Anim" true)
      (goto _label_2 :!via `Reset`))))

(event `Animation CounterClockwise`
  ; Planetary Gear Animation (Clockwise / Counter Clockwise)
  (`/Engine/EditorBlueprintResources/StandardMacros.DoOnce` false :!label _label_2
    (:`Completed`
      (`SkeletalMeshComponent.PlayAnimation` (`self.planetary_gears`) "/Game/Blueprints/PlanetaryGear/SkeletalMeshes/planetary_gears_AnimCounter.planetary_gears_AnimCounter" true))))

(event `Reset Do Once`
  ; Planetary Gear Animation (Clockwise / Counter Clockwise)
  (`|ExecutionSequence`
    (:`then_0`
      (goto _label_2 :!via `Reset`))
    (:`then_1`
      (goto _label :!via `Reset`))))

(fn `UserConstructionScript`)