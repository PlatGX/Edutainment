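; Earth axis display actor with ecliptic, celestial equator, rotational axis and Sun components, each group switchable on or off.
; Every Tick polls four IsHidden booleans and applies SetHiddenInGame to the matching meshes and labels.
; BeginPlay starts EarthTimeline, but its update drives nothing; the rotation calls and angle Lerp are left disconnected.
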(event `self.ReceiveBeginPlay`
  (`|ExecutionSequence`
    (:`then_0`
      (bind (_direction _newtrack_0) (`Timeline|Earth Timeline`)
        (:`Update`
          (`|ExecutionSequence`))))))

(event `self.ReceiveTick`
  (params (DeltaSeconds :type "Float (single-precision)"))
  (bind _sun (`self.Sun`))
  (bind _ecliptic (`self.Ecliptic`))
  (bind _celestial_equator (`self.Celestial Equator`))
  (bind _axis (`self.Axis`))
  (`|ExecutionSequence`
    (:`then_0`
      (if (`self.bIsEclipticHidden?`)
        (`SceneComponent.SetHiddenInGame` _ecliptic true false)
        (`SceneComponent.SetHiddenInGame` (`self.EclipticText`) true false)
        (else
          (`SceneComponent.SetHiddenInGame` _ecliptic false false)
          (`SceneComponent.SetHiddenInGame` (`self.EclipticText`) false false))))
    (:`then_1`
      (if (`self.bIsCelestialHidden?`)
        (`SceneComponent.SetHiddenInGame` _celestial_equator true false)
        (`SceneComponent.SetHiddenInGame` (`self.Celestial Equator Title`) true false)
        (`SceneComponent.SetHiddenInGame` (`self.TextRender`) true false)
        (`SceneComponent.SetHiddenInGame` (`self.Celestial Equator Text1`) true false)
        (`SceneComponent.SetHiddenInGame` (`self.Celestial Equator Text2`) true false)
        (`SceneComponent.SetHiddenInGame` (`self.Celestial Equator Arrow`) true false)
        (else
          (`SceneComponent.SetHiddenInGame` _celestial_equator false false)
          (`SceneComponent.SetHiddenInGame` (`self.Celestial Equator Title`) false false)
          (`SceneComponent.SetHiddenInGame` (`self.Celestial Equator Text2`) false false)
          (`SceneComponent.SetHiddenInGame` (`self.Celestial Equator Text1`) false false)
          (`SceneComponent.SetHiddenInGame` (`self.TextRender`) false false)
          (`SceneComponent.SetHiddenInGame` (`self.Celestial Equator Arrow`) false false))))
    (:`then_2`
      (if (`self.bIsRotationalAxisHidden?`)
        (`SceneComponent.SetHiddenInGame` _axis true false)
        (`SceneComponent.SetHiddenInGame` (`self.Axis Text`) true false)
        (else
          (`SceneComponent.SetHiddenInGame` _axis false false)
          (`SceneComponent.SetHiddenInGame` (`self.Axis Text`) false false))))
    (:`then_3`
      (if (`self.bIsSunHidden?`)
        (`SceneComponent.SetHiddenInGame` _sun true false)
        (else
          (`SceneComponent.SetHiddenInGame` _sun false false))))))

(fn `UserConstructionScript`)