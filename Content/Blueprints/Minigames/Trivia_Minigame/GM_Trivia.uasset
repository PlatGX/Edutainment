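; Game mode for the trivia minigame that runs categories of multiple-choice questions for all players.
; BeginCategory shuffles the category's question pool, then AskQuestion stores the correct answer, shuffles the choices and sends both question and choices to every PC_Trivia.
; PrepareNextQuestion advances the index and starts a timer, while AskQuestion calls EndRound once the question total is reached.
; Round flow is unfinished: StartRound only clears the category and question index, and EndRound just increments the round.
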(event `self.ReceiveBeginPlay`
  (`KismetSystemLibrary.PrintString` "WE ARE USING THIS GAME MODE" true true (struct :`R` 1.0 :`G` 0.009428 :`B` 0.229332 :`A` 1.0)))

(event `self.K2_PostLogin`
  (params (NewPlayer :type "PlayerController Object Reference"))
  (`KismetSystemLibrary.Delay` 3.0))

(event `BeginCategory`
  (params (Category :type "/Game/Data/MiniGames/TriviaQuestions/DA_Category Object Reference"))
  (bind _output_get (set `self.CurrentCategory` Category))
  (bind _output_get_2 (set `self.CurrentQuestionPool` (`/Game/Data/MiniGames/TriviaQuestions/DA_Category.QuestionPool` _output_get)))
  (`KismetArrayLibrary.Array_Shuffle` _output_get_2)
  (`self.AskQuestion`))

(event `AskQuestion`
  (bind _output (`|GetArrayItem` (`self.CurrentQuestionPool`) (`self.CurrentQuestionIndex`)))
  (bind _multiplechoice (`/Game/Data/MiniGames/TriviaQuestions/DA_Question.MultipleChoice` _output))
  (if (>= (`self.CurrentQuestionIndex`) (`self.TotalQuestions`))
    (`self.EndRound`)
    (else
      (set `self.CorrectAnswer` (`|GetArrayItem` _multiplechoice (`/Game/Data/MiniGames/TriviaQuestions/DA_Question.CorrectAnswer` _output)))
      (bind _output_get (set `self.CurrentMultipleChoice` _multiplechoice))
      (`KismetArrayLibrary.Array_Shuffle` _output_get)
      (for _array_element (`GameStateBase.PlayerArray` (`GameplayStatics.GetGameState`))
        (bind _aspc_trivia (cast `/Game/Blueprints/Minigames/Trivia_Minigame/PC_Trivia` (`PlayerState.GetPlayerController` _array_element)))
        (`/Game/Blueprints/Minigames/Trivia_Minigame/PC_Trivia.AskQuestion` _aspc_trivia (`|GetArrayItem` (`self.CurrentQuestionPool`) (`self.CurrentQuestionIndex`)) (`self.CurrentMultipleChoice`))))))

(fn `EndRound`
  (`/Engine/EditorBlueprintResources/StandardMacros.IncrementInt` (`self.CurrentRoundIndex`)))

(fn `PrepareNextQuestion`
  (`/Engine/EditorBlueprintResources/StandardMacros.IncrementInt` (`self.CurrentQuestionIndex`)
    (:`  `
      (`KismetSystemLibrary.K2_SetTimerDelegate` (`|CreateDelegate` :!event `AskQuestion`) 4.0))))

(fn `StartRound`
  (`|ExecutionSequence`
    (:`then_0`
      (set `self.CurrentCategory` null) ; Set New Category Here using the new category index
    )
    (:`then_1`
      (set `self.CurrentQuestionIndex` 0) ; Reset index to zero every round
    )))

(fn `UserConstructionScript`)