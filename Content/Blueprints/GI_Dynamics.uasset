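; Game instance for a dynamics game that holds the player's GPT conversation and persistent save data.
; SaveTranscript flattens user and assistant messages into a text file in the saved directory, then spawns a GPTSummarizer actor to summarize it.
; Init loads or creates save slots for a player UUID, appended once to the username, and for background music timestamp and play state.
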(event `UpdateTranscript`
  (params (GPTConversation :type "GPTChatPromptParams Structure"))
  (set `self.GPTConversation` GPTConversation))

(event `SaveTranscript`
  (for _array_element (`.Messages` (break `GPTChatPromptParams` (`self.GPTConversation`)))
    (bind ((`Role` _role) (`UserMessage` _usermessage) (`AssistantMessage` _assistantmessage)) (break `GPTChatMessage` _array_element))
    (switch `EGPTRole` _role
      (:`user`
        (bind (_role_2 _content) (break `UserMessage` _usermessage))
        (set `self.ConvoString` (`KismetStringLibrary.Concat_StrStr` (`self.ConvoString`) (`KismetStringLibrary.Concat_StrStr` _role_2 ": " (`.Content` (break `ContentPart` (`|GetArrayItem` _content))) " \n"))))
      (:`assistant`
        (bind ((`Role` _role_3) (`Content` _content_2)) (break `AssistantMessage` _assistantmessage))
        (set `self.ConvoString` (`KismetStringLibrary.Concat_StrStr` (`self.ConvoString`) (`KismetStringLibrary.Concat_StrStr` _role_3 ": " _content_2 " \n"))))))
  (`FileSDKBPLibrary.WriteStringToFile` (`KismetStringLibrary.Concat_StrStr` (`KismetSystemLibrary.GetProjectSavedDirectory`) "Transcript.txt") (`self.ConvoString`))
  (`self.GenerateSummary`))

(event `GenerateSummary`
  (bind _returnvalue (`|SpawnActorFromClass` "/Game/KalebsFolder/GPTSummarizer.GPTSummarizer_C" (`KismetMathLibrary.MakeTransform` (0.0 0.0 0.0)) "AlwaysSpawn" "MultiplyWithRoot" null null))
  (`/Game/KalebsFolder/GPTSummarizer.GenerateGPTSummary` _returnvalue (`self.ConvoString`)))

(event `AppendUUID`
  (`/Engine/EditorBlueprintResources/StandardMacros.DoOnce` false
    (:`Completed`
      (set `self.Username` (`KismetStringLibrary.Concat_StrStr` (`self.Username`) "_" (`/Game/Blueprints/SG_UUID.UUID` (`self.UUID_Save`)))))))

(event `self.ReceiveInit`
  (`|ExecutionSequence`
    (:`then_0`
      (bind _returnvalue (`GameplayStatics.DoesSaveGameExist` "UUID"))
      (if _returnvalue
        (bind _returnvalue_2 (`GameplayStatics.LoadGameFromSlot` "UUID"))
        (bind _assg_uuid (cast `/Game/Blueprints/SG_UUID` _returnvalue_2))
        (set `self.UUID_Save` _assg_uuid)
        (else
          (bind _returnvalue_3 (`GameplayStatics.CreateSaveGameObject` "/Game/Blueprints/SG_UUID.SG_UUID_C"))
          (bind _output_get (set `self.UUID_Save` _returnvalue_3))
          (set `/Game/Blueprints/SG_UUID.UUID` (`KismetGuidLibrary.Conv_GuidToString` (`KismetGuidLibrary.NewGuid`)) _output_get)
          (`GameplayStatics.SaveGameToSlot` _output_get "UUID"))))
    (:`then_1`
      ; BGM
      (bind _returnvalue_4 (`GameplayStatics.DoesSaveGameExist` "BGM"))
      (if _returnvalue_4
        (bind _returnvalue_5 (`GameplayStatics.LoadGameFromSlot` "BGM"))
        (bind _assg_bgm (cast `/Game/Blueprints/SG_BGM` _returnvalue_5))
        (set `self.BGM_Save` _assg_bgm)
        (else
          (bind _returnvalue_6 (`GameplayStatics.CreateSaveGameObject` "/Game/Blueprints/SG_BGM.SG_BGM_C"))
          (bind _output_get_2 (set `self.BGM_Save` _returnvalue_6))
          (`GameplayStatics.SaveGameToSlot` _output_get_2 "BGM"))))))

(event `SaveBGMTimestamp`
  (params (Timestamp :type "Float (double-precision)"))
  (bind _bgm_save (`self.BGM_Save`))
  ; BGM
  (set `/Game/Blueprints/SG_BGM.Timestamp` Timestamp _bgm_save)
  (`GameplayStatics.SaveGameToSlot` _bgm_save "BGM"))

(event `EraseBGMSave`
  (bind _bgm_save (`self.BGM_Save`))
  ; BGM
  (set `/Game/Blueprints/SG_BGM.Timestamp` 0.0 _bgm_save)
  (set `/Game/Blueprints/SG_BGM.Playing?` true _bgm_save)
  (`GameplayStatics.SaveGameToSlot` _bgm_save "BGM"))

(event `SaveBGMState`
  (params (`Playing?` :type Boolean))
  (bind _bgm_save (`self.BGM_Save`))
  ; BGM
  (set `/Game/Blueprints/SG_BGM.Playing?` `Playing?` _bgm_save)
  (`GameplayStatics.SaveGameToSlot` _bgm_save "BGM"))