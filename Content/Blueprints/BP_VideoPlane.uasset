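; BP_VideoPlane is a placeable plane that plays a media source as video in the world.
; The construction script creates a dynamic material instance on the plane, and BeginPlay assigns the media texture to its "MediaPlayer" parameter.
; After a brief delay it optionally scales the plane from Width and Height, applies the looping setting, then opens and plays the source on the media player.
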(event `self.ReceiveBeginPlay`
  (`self.SetMaterial`)
  (`KismetSystemLibrary.Delay` 0.01)
  (if (`self.OverrideScale?`)
    (`self.SetPlaneSize`))
  (`MediaPlayer.SetLooping` (`self.MediaPlayer`) (`self.ShouldLoop?`))
  (`self.PlayMedia`))

(event `SetMaterial`
  (`MaterialInstanceDynamic.SetTextureParameterValue` (`self.DynamicMI`) "MediaPlayer" (`self.MediaTexture`)))

(event `PlayMedia`
  (bind _mediaplayer (`self.MediaPlayer`))
  (`MediaPlayer.OpenSource` _mediaplayer (`self.MediaSource`))
  (`MediaPlayer.Play` _mediaplayer))

(event `SetPlaneSize`
  (`SceneComponent.SetWorldScale3D` (`self.Plane`) (`KismetMathLibrary.MakeVector` (/ (`self.Width`) 200.0) (/ (`self.Height`) 200.0) 1.0)))

(fn `UserConstructionScript`
  (bind _plane (`self.Plane`))
  (bind _returnvalue (`PrimitiveComponent.CreateDynamicMaterialInstance` _plane 0 (`PrimitiveComponent.GetMaterial` _plane 0) "MediaPlayer"))
  (set `self.DynamicMI` _returnvalue))