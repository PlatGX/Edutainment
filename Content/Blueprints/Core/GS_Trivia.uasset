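; GS_Trivia is the trivia game state that tracks each player's locked-in answer, time remaining, score and accuracy.
; MC_ events record or clear answers and times, and trigger AwardPoints with the correct answer.
; AwardPoints loops over players, playing right/wrong sounds, recording analytics, and scoring correct answers by time remaining.
; Its points broadcast takes TotalPoints from the score map's first entry, not the current player's.
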(event `MC_UpdateLockedInAnswers`
  (params (PlayerState :type "PlayerState Object Reference") (Answer :type Text) (TimeRemaining :type "Float (double-precision)"))
  (`BlueprintMapLibrary.Map_Add` (`self.LockedInAnswers`) PlayerState Answer) ; What did they answer
  (`BlueprintMapLibrary.Map_Add` (`self.PlayerTimes`) PlayerState TimeRemaining) ; How quick did they answer it
  (`self.OnAnswerSet` PlayerState Answer))

(event `MC_ClearLockedInAnswers`
  (`BlueprintMapLibrary.Map_Clear` (`self.LockedInAnswers`))
  (`BlueprintMapLibrary.Map_Clear` (`self.PlayerTimes`)))

(event `MC_AwardPoints`
  (params (CorrectAnswer :type Text) (QuestionNum :type Integer) (TriviaNum :type Integer))
  (`self.AwardPoints` CorrectAnswer QuestionNum TriviaNum))

(fn `AwardPoints`
  (params (`Correct Answer` :type Text) (QuestionNum :type Integer) (TriviaNum :type Integer))
  (locals (CorrectAnswer :type Text) (PlayerState :type "/Game/Blueprints/Core/PS_Trivia Object Reference"))
  (bind _playeraccuracy (`self.PlayerAccuracy`))
  (bind _playerstate (`local.PlayerState`))
  (bind _playerscores (`self.PlayerScores`))
  (bind _returnvalue (`KismetTextLibrary.EqualEqual_TextText` (`BlueprintMapLibrary.Map_Find` (`self.LockedInAnswers`) (`local.PlayerState`)) (`local.CorrectAnswer`)))
  (bind _returnvalue_2 (`KismetMathLibrary.Round` (* (`BlueprintMapLibrary.Map_Find` (`self.PlayerTimes`) (`local.PlayerState`)) 40.0)))
  (set `local.CorrectAnswer` `Correct Answer`)
  (for _array_element (`self.PlayerArray`)
    (bind _asps_trivia (cast `/Game/Blueprints/Core/PS_Trivia` _array_element))
    (set `local.PlayerState` _asps_trivia)
    (`GameplayStatics.PlaySound2D` (select `bool` _returnvalue :`false` "/Game/SFX/SW_WrongAnswer.SW_WrongAnswer" :`true` "/Game/SFX/SW_CorrectAnswer.SW_CorrectAnswer" :!type "SoundBase Object Reference") 1.0 1.0 0.0 null null)
    (`self.SendAnalytic` (`local.QuestionNum`) (`local.TriviaNum`) _returnvalue)
    (if _returnvalue
      (`BlueprintMapLibrary.Map_Add` _playerscores (`local.PlayerState`) (+ (`BlueprintMapLibrary.Map_Find` _playerscores (`local.PlayerState`)) _returnvalue_2))
      (`/Game/Blueprints/Core/PS_Trivia.OnPointsAwarded_Event` (`local.PlayerState`) _returnvalue_2)
      (`self.OnPointsAwarded` _returnvalue_2 (`.Value` (`BlueprintMapLibrary.Map_GetKeyValueByIndex` (`self.PlayerScores`))) (`local.PlayerState`))
      (`BlueprintMapLibrary.Map_Add` _playeraccuracy _playerstate (+ (`BlueprintMapLibrary.Map_Find` _playeraccuracy _playerstate) 1)))))

(fn `SendAnalytic`
  (params (QuestionNum :type Integer) (TriviaNum :type Integer) (Correct :type Boolean))
  (`GoogleAnalyticsMPStatics.RecordNamedEvent` (`KismetTextLibrary.Conv_TextToString` (`|FormatText` "L{l}:Q{q}" TriviaNum QuestionNum)) (`|MakeMap` "ep.Trivia_Correct" (`KismetMathLibrary.SelectString` "Correct" "Incorrect" Correct))))

(fn `UserConstructionScript`)