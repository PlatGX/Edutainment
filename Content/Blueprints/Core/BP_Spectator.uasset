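; BP_Spectator is a game mode, judging by its login and logout events, that tracks connected players and shares the user list with them.
; PostLogin and OnLogout add or remove controllers, then call UpdatePlayerListGM.
; That function rebuilds the SUser list from PlayerState names, with points and level as zeroed placeholders.
; It then pushes the full list to each BP_PlayerController through UpdateUserListPC.
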(event `self.ReceiveBeginPlay`)

(event `self.K2_PostLogin`
  (params (NewPlayer :type "PlayerController Object Reference"))
  ;[0.001989 1 0 0.5] Test - WORKING
  (`KismetArrayLibrary.Array_Add` (`self.PlayerControllerList`) NewPlayer)
  (`self.UpdatePlayerListGM` :!label _label))

(event `self.K2_OnLogout`
  (params (ExitingController :type "Controller Object Reference"))
  ;[0.001989 1 0 0.5] Test - WORKING
  (bind _asplayer_controller (cast `PlayerController` ExitingController))
  (`KismetArrayLibrary.Array_RemoveItem` (`self.PlayerControllerList`) _asplayer_controller)
  (goto _label))

(fn `UpdatePlayerListGM`
  ;[0 1 0 0.5] Test - WORKING
  (`KismetArrayLibrary.Array_Clear` (`self.UserList`))
  (for _array_element (`self.PlayerControllerList`)
    (`KismetArrayLibrary.Array_Add` (`self.UserList`) (make `/Game/Widgets/Leaderboards/SUser` (`KismetTextLibrary.Conv_StringToText` (`PlayerState.GetPlayerName` (`Controller.PlayerState` _array_element))))))
  (for _array_element_2 (`self.PlayerControllerList`)
    (bind _asbp_player_controller (cast `/Game/Blueprints/Core/BP_PlayerController` _array_element_2))
    (`/Game/Blueprints/Core/BP_PlayerController.UpdateUserListPC` _asbp_player_controller (`self.UserList`))))

(fn `UserConstructionScript`)