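; Player controller that sets up background music, input and leaderboard widgets, handles pausing, and relays trivia rounds.
; IA_Pause toggles the pause menu outside the main menu, pausing and resuming the video player widget too.
; Questions start a timer and reach HUD_Trivia, answers go to GS_Trivia, and timer expiry checks all players before GM_Trivia prepares the next question.
; Leaderboard updates retry until the widget reference is valid.
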(event `self.ReceiveBeginPlay`
  (`|ExecutionSequence`
    (:`then_0`
      (`KismetSystemLibrary.Delay` 0.2)
      (bind _returnvalue (`|CreateWidget` "/Game/Widgets/MainMenu/WBP_BGM.WBP_BGM_C" (`GameplayStatics.GetPlayerController` 0)))
      (bind _output_get (set `self.W_BGM` _returnvalue))
      (`UserWidget.AddToViewport` _output_get 1))
    (:`then_1`
      (bind _asbp_player_controller (cast `/Game/Blueprints/Core/BP_PlayerController` (`GameplayStatics.GetPlayerController` 0)))
      (message `EnhancedInputSubsystemInterface.AddMappingContext` (pcsubsystem `EnhancedInputLocalPlayerSubsystem` _asbp_player_controller) "/Game/Blueprints/Core/Inputs/IMC_default.IMC_default" 0 (struct))
      (`KismetSystemLibrary.PrintString` "mapping context added")
      (`WidgetBlueprintLibrary.SetInputMode_GameAndUIEx` self null))
    (:`then_2`
      (`self.SetUpLeaderboards`))))

(event `/Game/Blueprints/BPI_WidgetInteractions.PauseMenu`
  (bind _pauseref (`self.PauseRef`))
  (`KismetSystemLibrary.Delay` 0.2 :!label _label)
  (bind _returnvalue (`GameplayStatics.GetCurrentLevelName` true))
  (if (not (`KismetStringLibrary.EqualEqual_StrStr` _returnvalue "00_Main_Menu_Current"))
    (if (not (`GameplayStatics.IsGamePaused`))
      (bind _returnvalue_2 (`|CreateWidget` "/Game/Widgets/WBP_PauseMenu.WBP_PauseMenu_C" (`GameplayStatics.GetPlayerController` 0)))
      (bind _output_get (set `self.PauseRef` _returnvalue_2))
      (`UserWidget.AddToViewport` _output_get 0)
      (bind _returnvalue_3 (`VictoryBPFunctionLibrary.GetFirstWidgetOfClass` "/Game/Widgets/VideoPlayer/WBP_UpdatedVideoPlayer.WBP_UpdatedVideoPlayer_C"))
      (`/Game/Blueprints/BPI_WidgetInteractions.PauseVideo` _returnvalue_3)
      (`GameplayStatics.SetGamePaused` true)
      (else
        (`/Engine/EditorBlueprintResources/StandardMacros.DoOnce` false :!label _label_2
          (:`Completed`
            (`/Engine/EditorBlueprintResources/StandardMacros.IsValid` _pauseref
              (:`Is Valid`
                (`/Game/Widgets/WBP_PauseMenu.FadeOffUI` _pauseref)
                (`KismetSystemLibrary.Delay` 0.5)
                (`Widget.RemoveFromParent` _pauseref))
              (:`Is Not Valid`
                _))
            (`GameplayStatics.SetGamePaused` false)
            (bind _returnvalue_4 (`VictoryBPFunctionLibrary.GetFirstWidgetOfClass` "/Game/Widgets/VideoPlayer/WBP_UpdatedVideoPlayer.WBP_UpdatedVideoPlayer_C"))
            (`/Game/Blueprints/BPI_WidgetInteractions.PlayVideo` _returnvalue_4)
            (goto _label_2 :!via `Reset`)))))))

(event `EnhancedInput|/Game/Blueprints/Core/Inputs/IA_Pause`
  (params (ActionValue :type Boolean) (ElapsedSeconds :type "Float (double-precision)") (TriggeredSeconds :type "Float (double-precision)") (InputAction :type "InputAction Object Reference" :default "/Game/Blueprints/Core/Inputs/IA_Pause.IA_Pause"))
  (:`Triggered`
    (goto _label)))

(event `AskQuestion`
  (params (Question :type "/Game/Data/MiniGames/TriviaQuestions/DA_Question Object Reference") (MultipleChoice :type "Array of Text"))
  ; Trivia
  (`self.StartTimer`)
  (bind _ashud_trivia (cast `/Game/Blueprints/Core/HUD_Trivia` (`self.GetHUD`)))
  (`/Game/Blueprints/Core/HUD_Trivia.AskQuestion` _ashud_trivia Question MultipleChoice))

(event `UpdateUserListPC`
  (params (UserList :type "Array of /Game/Widgets/Leaderboards/SUserInfo Structure"))
  (bind _leaderboardhud_ref (`self.LeaderboardHUD_Ref`))
  ;[0 1 0 0.5] Test - WORKING
  (`/Engine/EditorBlueprintResources/StandardMacros.IsValid` _leaderboardhud_ref :!label _label_3
    (:`Is Valid`
      (`/Game/Widgets/Leaderboards/WBP_LeaderboardsHUD.UpdatePlayerList` _leaderboardhud_ref UserList))
    (:`Is Not Valid`
      (`KismetSystemLibrary.Delay` 0.1)
      (goto _label_3))))

(event `SetAnswer`
  (params (Answer :type Text) (TimeRemaining :type "Float (double-precision)"))
  ; Trivia
  (bind _asgs_trivia (cast `/Game/Blueprints/Core/GS_Trivia` (`GameplayStatics.GetGameState`)))
  (`/Game/Blueprints/Core/GS_Trivia.MC_UpdateLockedInAnswers` _asgs_trivia (`self.PlayerState`) Answer TimeRemaining))

(event `TimerExpired`
  ; Trivia
  (bind _return (`self.CheckTimerStatus`))
  (if _return
    (bind _asgm_trivia (cast `/Game/Blueprints/Minigames/Trivia_Minigame/GM_Trivia` (`GameplayStatics.GetGameMode`)))
    (`self.CLIENT_RevealAnswers` (`/Game/Blueprints/Minigames/Trivia_Minigame/GM_Trivia.CorrectAnswer` _asgm_trivia))
    (`/Game/Blueprints/Minigames/Trivia_Minigame/GM_Trivia.PrepareNextQuestion` _asgm_trivia)))

(event `CLIENT_RevealAnswers`
  (params (`Correct Answer` :type Text))
  ; Trivia
  (bind _ashud_trivia (cast `/Game/Blueprints/Core/HUD_Trivia` (`self.GetHUD` (`GameplayStatics.GetPlayerController` 0))))
  (`/Game/Blueprints/Core/HUD_Trivia.RevealAnswers` _ashud_trivia `Correct Answer`))

(fn `CheckTimerStatus`
  (returns (Return :type Boolean))
  (for _array_element (`GameStateBase.PlayerArray` (`GameplayStatics.GetGameState`))
    (bind _aspc_trivia (cast `/Game/Blueprints/Minigames/Trivia_Minigame/PC_Trivia` (`PlayerState.GetPlayerController` _array_element)))
    (if (`KismetSystemLibrary.K2_IsTimerActiveHandle` (`/Game/Blueprints/Minigames/Trivia_Minigame/PC_Trivia.QuestionTimer` _aspc_trivia))
      (return false)))
  (return true))

(fn `SetUpLeaderboards`
  ;[0.02675 1 0.000352 0.5] Test - WORKING
  (if (`self.IsLocalController`)
    (bind _returnvalue (`|CreateWidget` "/Game/Widgets/Leaderboards/WBP_LeaderboardsHUD.WBP_LeaderboardsHUD_C"))
    (set `self.LeaderboardHUD_Ref` _returnvalue)))

(fn `StartTimer`
  (bind _returnvalue (`KismetSystemLibrary.K2_SetTimerDelegate` (`|CreateDelegate` :!event `TimerExpired`) 20.0))
  (set `self.QuestionTimer` _returnvalue))

(fn `UserConstructionScript`)