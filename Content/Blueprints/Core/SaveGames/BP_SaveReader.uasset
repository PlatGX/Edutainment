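; BP_SaveReader exports a value from the PlayerStats save game to a text file, apparently as a developer utility.
; On BeginPlay it loads that slot if it exists, casts it to SG_PlayerStats and stores the reference.
; It then writes the Score field, labelled as "UUID", to SaveGameData in a hard-coded desktop folder, allowing overwrite.
; The save's actual UUID field is left unused.
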(event `self.ReceiveBeginPlay`
  (bind _returnvalue (`GameplayStatics.DoesSaveGameExist` "PlayerStats"))
  (if _returnvalue
    (bind _returnvalue_2 (`GameplayStatics.LoadGameFromSlot` "PlayerStats"))
    (bind _assg_player_stats (cast `/Game/Blueprints/Core/SaveGames/SG_PlayerStats` _returnvalue_2))
    (bind _output_get (set `self.SaveRef` _assg_player_stats))
    (`VictoryBPFunctionLibrary.FileIO__SaveStringTextToFile` "C:\\Users\\samue\\Desktop\\SaveData" "SaveGameData" (`KismetTextLibrary.Conv_TextToString` (`|FormatText` "UUID: {st}" (`KismetStringLibrary.Conv_IntToString` (`/Game/Blueprints/Core/SaveGames/SG_PlayerStats.Score` _output_get)))) true)))

(fn `UserConstructionScript`)