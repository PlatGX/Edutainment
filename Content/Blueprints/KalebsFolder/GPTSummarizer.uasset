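; Summarizes a conversation through GPT when the game is quitting, then saves and uploads the result.
; GenerateGPTSummary adds the conversation as a user message and sends the request through the AIITK component.
; On completion it writes the summary to the saved directory and sends it, joined with the conversation, under the GI_Dynamics username using a hardcoded API key.
; Both upload success and failure quit the game after a short delay.
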(event `GenerateGPTSummary`
  (params (Content :type String))
  (bind _gptrequest (`self.GPTRequest`))
  (bind _output_get (set `self.Conversation` Content))
  (`KismetArrayLibrary.Array_AddUnique` (`.Messages` (break `GPTChatPromptParams` _gptrequest)) (make `GPTChatMessage` :`Role` "user" :`UserMessage` (make `UserMessage` (`|MakeArray` (make `ContentPart` "Text" _output_get) :!type "ContentPart Structure"))))
  (`/AIIntegrationToolkit/Core/Components/AIITKComponentBP.SendRequestToGPT` (`self.AIITKComponentBP`) _gptrequest))

(event `self.AIITKComponentBP.OnGPTCompleted`
  (params (Completion :type "GPTChatCompletion Structure"))
  (bind _output_get (set `self.Summary` (`.Content` (break `AssistantMessage` (`.AssistantMessage` (break `GPTChatMessage` (`.Message` (break `GPTChatChoice` (`|GetArrayItem` Completion_Choices)))))))))
  (`FileSDKBPLibrary.WriteStringToFile` (`KismetStringLibrary.Concat_StrStr` (`KismetSystemLibrary.GetProjectSavedDirectory`) "Summary.txt") _output_get)
  (bind _asgi_dynamics (cast `/Game/Blueprints/Core/GI_Dynamics` (`GameplayStatics.GetGameInstance`)))
  (bind _structout (setmembers `AIITK_NTK_JsonHttpRequestConfig` :`StructRef` (`self.TranscriptUpdateRequest`) :`Body` (`AIITK_NTK_JsonHttpFunctionLibrary.ConvertStructToJsonString` (make `/Game/Data/TranscriptData/TranscriptData` (`/Game/Blueprints/Core/GI_Dynamics.Username` _asgi_dynamics) (`KismetStringLibrary.Concat_StrStr` (`self.Summary`) " \n \n \n" (`self.Conversation`))))))
  ;[0 0 0 0.5] Should probs use encrypted storage here but no one else was using it
  (`BlueprintMapLibrary.Map_Add` (`.Headers` (break `AIITK_NTK_JsonHttpRequestConfig` _structout)) "x-api-key" "sk_live_NGep5LcDfvvQeTcOXTmvDQymeF4DpbZr")
  (`AIITK_NTK_JsonHttpFunctionLibrary.SendHttpRequestWithConfig` :`RequestConfig` (`self.TranscriptUpdateRequest`) :`OnError` (delegate `TranscriptError`) :`OnComplete` (delegate `TranscriptUpdated`)))

(event `TranscriptUpdated`
  (params (ResponseData :type String))
  ;[0 0 0 0.5] This should really be an interface call back to the GI or something but we'll just go ahead and quit since the summary is only ever generated when quitting -KK
  (`KismetSystemLibrary.Delay` 0.2 :!label _label)
  (`KismetSystemLibrary.QuitGame` null "Quit"))

(event `TranscriptError`
  (params (ErrorMessage :type String))
  (goto _label))

(fn `UserConstructionScript`)