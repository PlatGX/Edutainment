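; BP_SpawnProceduralArrows is a helper actor that spawns procedural BP_ArrowIndicator arrows between a given start and end point with a given material.
; CreateArrow spawns the indicator at this actor's transform through NewArrow, configures it with SetParams and returns it.
; SetParams applies fixed settings for a zero-height, zero-speed, unfaded arrow with custom segment and head meshes, deferring the rebuild to a final ForceUpdate.
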(fn `CreateArrow`
  (params (Start :type "Vector Structure") (End :type "Vector Structure") (Material :type "Material Object Reference"))
  (returns (Arrow :type "/Game/ProceduralArrow/Blueprints/BP_ArrowIndicator Object Reference"))
  (bind _arrow (`self.NewArrow`))
  (`self.SetParams` _arrow Start End Material)
  (return _arrow))

(fn `NewArrow`
  (returns (Arrow :type "/Game/ProceduralArrow/Blueprints/BP_ArrowIndicator Object Reference"))
  (bind _returnvalue (`|SpawnActorFromClass` "/Game/ProceduralArrow/Blueprints/BP_ArrowIndicator.BP_ArrowIndicator_C" (`self.GetTransform`) "Undefined" "MultiplyWithRoot" null null))
  (return _returnvalue))

(fn `SetParams`
  (params (Arrow :type "/Game/ProceduralArrow/Blueprints/BP_ArrowIndicator Object Reference") (StartVector :type "Vector Structure") (EndVector :type "Vector Structure") (Material :type "Material Object Reference"))
  (`/Game/ProceduralArrow/Blueprints/BP_ArrowIndicator.SetMaxHeight` Arrow 0.0 false)
  (`/Game/ProceduralArrow/Blueprints/BP_ArrowIndicator.SetDistanceBetweenSegment` Arrow 5.0 false)
  (`/Game/ProceduralArrow/Blueprints/BP_ArrowIndicator.SetStart` Arrow StartVector)
  (`/Game/ProceduralArrow/Blueprints/BP_ArrowIndicator.SetEnd` Arrow EndVector)
  (`/Game/ProceduralArrow/Blueprints/BP_ArrowIndicator.SetStartEnd` Arrow StartVector EndVector)
  (`/Game/ProceduralArrow/Blueprints/BP_ArrowIndicator.SetSpeed` Arrow 0.0)
  (`/Game/ProceduralArrow/Blueprints/BP_ArrowIndicator.SetFadeDistance` Arrow 0.0 false)
  (`/Game/ProceduralArrow/Blueprints/BP_ArrowIndicator.SetSegmentsMesh` Arrow "/Game/ProceduralArrow/Meshes/SM_ArrowSegment2.SM_ArrowSegment2")
  (`/Game/ProceduralArrow/Blueprints/BP_ArrowIndicator.SetSegmentsMaterial` Arrow Material)
  (`/Game/ProceduralArrow/Blueprints/BP_ArrowIndicator.SetHeadMesh` Arrow "/Game/ProceduralArrow/Meshes/CustomArrowHead.CustomArrowHead")
  (`/Game/ProceduralArrow/Blueprints/BP_ArrowIndicator.SetHeadMaterial` Arrow Material)
  (`/Game/ProceduralArrow/Blueprints/BP_ArrowIndicator.SetSegmentOffset` Arrow 4.0 10.0 false)
  (`/Game/ProceduralArrow/Blueprints/BP_ArrowIndicator.ForceUpdate` Arrow))

(fn `UserConstructionScript`)