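; BP_FileCreator logs messages to a per-player transcript text file named after the saved Username in GI_Dynamics.
; UpdateFile loads the file's lines, adds the message and saves the whole array with both overwrite and append enabled.
; GetDirectory returns the project directory, or its parent folder when packaged for distribution, and prints the chosen path.
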(fn `GetDirectory`
  (returns (ReturnValue :type String))
  (bind _returnvalue (`KismetSystemLibrary.GetProjectDirectory`))
  (bind _returnvalue_2 (`KismetSystemLibrary.GetProjectDirectory`))
  (bind _returnvalue_3 (`KismetStringLibrary.GetSubstring` _returnvalue_2 0 (- (`KismetStringLibrary.Len` _returnvalue_2) 1)))
  (bind _returnvalue_4 (`KismetStringLibrary.GetSubstring` _returnvalue_3 0 (+ (`KismetStringLibrary.FindSubstring` _returnvalue_3 "/" false true) 1)))
  (if (`KismetSystemLibrary.IsPackagedForDistribution`)
    (`KismetSystemLibrary.PrintString` _returnvalue_4)
    (return _returnvalue_4)
    (else
      (`KismetSystemLibrary.PrintString` _returnvalue)
      (return _returnvalue))))

(fn `UpdateFile`
  (params (Message :type String))
  (bind _returnvalue (`self.GetDirectory`))
  (bind _playerstats_save (`/Game/Blueprints/Core/GI_Dynamics.PlayerStats_Save` (cast `/Game/Blueprints/Core/GI_Dynamics` (`GameplayStatics.GetGameInstance`) :!pure true)))
  (bind _output_get (set `self.Transcript` (`VictoryBPFunctionLibrary.LoadStringArrayFromFile` (`KismetStringLibrary.Concat_StrStr` _returnvalue (`KismetStringLibrary.Concat_StrStr` (`/Game/Blueprints/Core/SaveGames/SG_PlayerStats.Username` _playerstats_save) ".txt")))))
  (`KismetArrayLibrary.Array_Add` _output_get Message)
  (`VictoryBPFunctionLibrary.FileIO__SaveStringArrayToFile` _returnvalue (`KismetStringLibrary.Concat_StrStr` (`/Game/Blueprints/Core/SaveGames/SG_PlayerStats.Username` _playerstats_save) ".txt") (`self.Transcript`) true true))