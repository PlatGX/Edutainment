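; Procedural arrow indicator actor that draws an arched trail of mesh segments with a head, from its location to a settable end point.
; A three-point spline, its height capped by MaxHeight, positions both segments and head, while Tick scrolls the segments at the configured speed.
; Middle segments share an instanced mesh; fading end segments use pooled static mesh components with per-mesh dynamic opacity.
; Setters change endpoints and configuration at runtime.
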(event EventTick
  (params (DeltaSeconds :type Float%20%28single-precision%29))
  (if (CallFunction|NeedUpdateDuringTick)
    (Variables|Default|SetTimeOffset (Math|Float|%(Float) (+ (Variables|Default|GetTimeOffset) (* DeltaSeconds (Utilities|Struct|BreakFArrowIndicator_SegmentsConfig (Variables|Arrow|GetSegments)))) (Utilities|Struct|BreakFArrowIndicator_SegmentsConfig (Variables|Arrow|GetSegments))))
    (Update|ForceUpdate)))

(fn ConstructionScript
  (bind _head (Variables|Arrow|GetHead))
  (bind _segments (Variables|Arrow|GetSegments))
  (bind _segmentsmaterial (Utilities|Struct|BreakFArrowIndicator_SegmentsConfig _segments))
  (bind _headmaterial (Utilities|Struct|BreakFArrowIndicator_HeadConfig _head))
  (Utilities|FlowControl|Sequence
    (:then_0
      ;[1 1 1] Create spline component
      (bind _returnvalue (AddComponent|AddSplineComponent false))
      (Variables|Default|SetSpline _returnvalue)
      (Update|UpdateSpline))
    (:then_1
      ;[1 1 1] Create segments component and add child if needed
      (Utilities|IsValid (Utilities|Struct|BreakFArrowIndicator_SegmentsConfig (Variables|Arrow|GetSegments))
        (:Is%20Valid
          (bind _returnvalue_2 (AddComponent|AddInstancedStaticMeshComponent false))
          (bind _output_get (Variables|Default|SetSegmentsMeshInstance _returnvalue_2))
          (Components|StaticMesh|SetStaticMesh _output_get (Utilities|Struct|BreakFArrowIndicator_SegmentsConfig (Variables|Arrow|GetSegments)))
          (Collision|SetCollisionEnabled (Variables|Default|GetSegmentsMeshInstance) "NoCollision")
          (Utilities|IsValid _segmentsmaterial
            (:Is%20Valid
              (bind _returnvalue_3 (Rendering|Material|CreateDynamicMaterialInstance _segmentsmaterial "None" "None" :!class /Script/Engine.KismetMaterialLibrary))
              (Rendering|Material|SetMaterial (Variables|Default|GetSegmentsMeshInstance) 0 _returnvalue_3))))))
    (:then_2
      ;[1 1 1] Create head mesh
      (Utilities|IsValid (Utilities|Struct|BreakFArrowIndicator_HeadConfig (Variables|Arrow|GetHead))
        (:Is%20Valid
          (bind _returnvalue_4 (AddComponent|AddStaticMeshComponent false))
          (bind _output_get_2 (Variables|Default|SetHeadMeshInstance _returnvalue_4))
          (Components|StaticMesh|SetStaticMesh _output_get_2 (Utilities|Struct|BreakFArrowIndicator_HeadConfig (Variables|Arrow|GetHead)))
          (Collision|SetCollisionEnabled (Variables|Default|GetHeadMeshInstance) "NoCollision")
          (Utilities|IsValid _headmaterial
            (:Is%20Valid
              (bind _returnvalue_5 (Rendering|Material|CreateDynamicMaterialInstance _headmaterial "None" "None" :!class /Script/Engine.KismetMaterialLibrary))
              (Rendering|Material|SetMaterial (Variables|Default|GetHeadMeshInstance) 0 _returnvalue_5))))))
    (:then_3
      ;[1 1 1] Update arrow
      (Update|UpdateSegments)
      (Update|UpdateHead))))

(fn GetFadeOpacity
  (params (Offset :type Float%20%28double-precision%29) (SplineLenght :type Float%20%28double-precision%29))
  (if (< Offset (Utilities|Struct|BreakFArrowIndicator_SegmentsConfig (Variables|Arrow|GetSegments)))
    (return (/ Offset (Utilities|Struct|BreakFArrowIndicator_SegmentsConfig (Variables|Arrow|GetSegments))))
    (else
      (return (/ (- SplineLenght Offset) (Utilities|Struct|BreakFArrowIndicator_SegmentsConfig (Variables|Arrow|GetSegments)))))))

(fn GetSegmentTransform
  (params (Distance :type Float%20%28double-precision%29) (InTransform :type Transform))
  (return (Math|Transform|ComposeTransforms InTransform (Spline|GetTransformatDistanceAlongSpline (Variables|Default|GetSpline) (Math|Float|Clamp(Float) Distance 0.0001 (- (Spline|GetSplineLength (Variables|Default|GetSpline)) 0.0001)) "Local" false))))

(fn ClearUnusedInstancedSegments
  (params (UsedSegments :type Integer))
  (if (> (Components|InstancedStaticMesh|GetInstanceCount (Variables|Default|GetSegmentsMeshInstance)) UsedSegments)
    (for _index (range UsedSegments (- (Components|InstancedStaticMesh|GetInstanceCount (Variables|Default|GetSegmentsMeshInstance)) 1))
      (Class|InstancedStaticMeshComponent|RemoveInstance (Variables|Default|GetSegmentsMeshInstance) _index))))

(fn ClearUnusedStaticSegments
  (params (UsedSegments :type Integer))
  (if (< UsedSegments (Utilities|Array|Length (Variables|Default|GetFadedSegments)))
    (for _index (range UsedSegments (Utilities|Array|LastIndex (Variables|Default|GetFadedSegments)))
      (Development|SetHiddeninGame (Utilities|Array|Get(acopy) (Variables|Default|GetFadedSegments) _index) true false))))

(fn SetSegmentsMesh
  (params (SegmentsMesh :type Static%20Mesh%20Object%20Reference))
  (bind _segments (Variables|Arrow|GetSegments))
  (bind _segmentsmaterial (Utilities|Struct|BreakFArrowIndicator_SegmentsConfig _segments))
  (Utilities|IsValid SegmentsMesh
    (:Is%20Valid
      (Utilities|Struct|SetmembersinFArrowIndicator_SegmentsConfig (Variables|Arrow|GetSegments) SegmentsMesh)
      (Utilities|IsValid (Variables|Default|GetSegmentsMeshInstance)
        (:Is%20Valid
          (Components|StaticMesh|SetStaticMesh (Variables|Default|GetSegmentsMeshInstance) SegmentsMesh))
        (:Is%20Not%20Valid
          (bind _returnvalue (AddComponent|AddInstancedStaticMeshComponent false))
          (bind _output_get (Variables|Default|SetSegmentsMeshInstance _returnvalue))
          (Components|StaticMesh|SetStaticMesh _output_get (Utilities|Struct|BreakFArrowIndicator_SegmentsConfig (Variables|Arrow|GetSegments)))
          (Collision|SetCollisionEnabled (Variables|Default|GetSegmentsMeshInstance) "NoCollision")
          (Utilities|IsValid _segmentsmaterial
            (:Is%20Valid
              (bind _returnvalue_2 (Rendering|Material|CreateDynamicMaterialInstance _segmentsmaterial "None" "None" :!class /Script/Engine.KismetMaterialLibrary))
              (Rendering|Material|SetMaterial (Variables|Default|GetSegmentsMeshInstance) 0 _returnvalue_2))))))))

(fn SetSegmentsMaterial
  (params (SegmentsMaterial :type Material%20Interface%20Object%20Reference))
  (Utilities|IsValid SegmentsMaterial
    (:Is%20Valid
      (Utilities|Struct|SetmembersinFArrowIndicator_SegmentsConfig (Variables|Arrow|GetSegments) SegmentsMaterial)
      (Utilities|IsValid (Variables|Default|GetSegmentsMeshInstance)
        (:Is%20Valid
          (bind _returnvalue (Rendering|Material|CreateDynamicMaterialInstance SegmentsMaterial "None" "None" :!class /Script/Engine.KismetMaterialLibrary))
          (Rendering|Material|SetMaterial (Variables|Default|GetSegmentsMeshInstance) 0 _returnvalue))))))

(fn SetDistanceBetweenSegment
  (params (DistanceBetweenSegment :type Float%20%28double-precision%29) (bForceUpdate :type Boolean))
  (Utilities|Struct|SetmembersinFArrowIndicator_SegmentsConfig (Variables|Arrow|GetSegments) DistanceBetweenSegment)
  (if bForceUpdate
    (Update|UpdateSegments)))

(fn UpdateSpline
  (bind _endposition (Variables|Arrow|GetEndPosition))
  (Spline|ClearSplinePoints (Variables|Default|GetSpline) false)
  (Class|SplineComponent|AddPoint (Variables|Default|GetSpline) (Utilities|Struct|MakeSplinePoint 0.0 "0.000000,0.000000,0.000000" "0.000000,0.000000,0.000000" "0.000000,0.000000,0.000000" "0.000000,0.000000,0.000000" "1.000000,1.000000,1.000000" "CurveClamped") false)
  (Class|SplineComponent|AddPoint (Variables|Default|GetSpline) (Utilities|Struct|MakeSplinePoint 1.0 (|((Vector(0,0,(min(((VectorLength(end_position))/2),max_height))))+(end_position/2)) (Variables|Arrow|GetEndPosition) (Utilities|Struct|BreakFArrowIndicator_SegmentsConfig (Variables|Arrow|GetSegments))) _endposition _endposition "0.000000,0.000000,0.000000" "1.000000,1.000000,1.000000" "CurveCustomTangent") false)
  (Class|SplineComponent|AddPoint (Variables|Default|GetSpline) (Utilities|Struct|MakeSplinePoint 2.0 (Variables|Arrow|GetEndPosition) "0.000000,0.000000,0.000000" "0.000000,0.000000,0.000000" "0.000000,0.000000,0.000000" "1.000000,1.000000,1.000000" "CurveClamped") true))

(fn UpdateSegments
  (bind _segments (Variables|Arrow|GetSegments))
  (bind _segments_2 (Variables|Arrow|GetSegments))
  (bind _segments_3 (Variables|Arrow|GetSegments))
  (bind _segments_4 (Variables|Arrow|GetSegments))
  (bind _segments_5 (Variables|Arrow|GetSegments))
  (bind (_minfade _maxfade) (Utilities|Struct|BreakFArrowIndicator_SegmentsConfig _segments_5))
  (bind (_finalsegmentoffset _bincludeheadfinaloffset) (Utilities|Struct|BreakFArrowIndicator_SegmentsConfig _segments_3))
  (bind (_distancebetweensegment _fadedistance) (Utilities|Struct|BreakFArrowIndicator_SegmentsConfig _segments_4))
  (bind _distancebetweensegment_2 (Utilities|Struct|BreakFArrowIndicator_SegmentsConfig _segments))
  (bind (_transformsegment _initialsegmentoffset) (Utilities|Struct|BreakFArrowIndicator_SegmentsConfig _segments_2))
  (Utilities|IsValid (Variables|Default|GetSegmentsMeshInstance)
    (:Is%20Valid
      (bind _output_get (LocalVariables|SetSplineLenght (- (- (Spline|GetSplineLength (Variables|Default|GetSpline)) (Utilities|Struct|BreakFArrowIndicator_SegmentsConfig (Variables|Arrow|GetSegments))) (Math|Float|SelectFloat (+ (Utilities|Struct|BreakFArrowIndicator_HeadConfig (Variables|Arrow|GetHead)) _finalsegmentoffset) _finalsegmentoffset _bincludeheadfinaloffset))))
      (if (> _output_get 0.0)
        (LocalVariables|SetCumulativeOffset (Math|Float|Clamp(Float) (Math|Float|%(Float) (Variables|Default|GetTimeOffset) _distancebetweensegment_2) 0.01 _distancebetweensegment_2))
        (LocalVariables|SetCurrentInstancedCount (Components|InstancedStaticMesh|GetInstanceCount (Variables|Default|GetSegmentsMeshInstance)))
        (while (< (LocalVariables|GetCumulativeOffset) (LocalVariables|GetSplineLenght))
          (LocalVariables|SetCurrentSegmentTransform (Segments|GetSegmentTransform (+ (LocalVariables|GetCumulativeOffset) _initialsegmentoffset) _transformsegment))
          (if (or (< (LocalVariables|GetCumulativeOffset) (Utilities|Struct|BreakFArrowIndicator_SegmentsConfig (Variables|Arrow|GetSegments))) (> (LocalVariables|GetCumulativeOffset) (- (LocalVariables|GetSplineLenght) (Utilities|Struct|BreakFArrowIndicator_SegmentsConfig (Variables|Arrow|GetSegments)))))
            (if (> (+ (LocalVariables|GetFadedSegmentIndex) 1) (Utilities|Array|Length (Variables|Default|GetFadedSegments)))
              (Utilities|IsValid (Utilities|Struct|BreakFArrowIndicator_SegmentsConfig (Variables|Arrow|GetSegments))
                (:Is%20Valid
                  (bind _returnvalue (AddComponent|AddStaticMeshComponent false (LocalVariables|GetCurrentSegmentTransform)))
                  (bind _output_get_2 (LocalVariables|SetCurrentSelectedMesh _returnvalue))
                  (Collision|SetCollisionEnabled _output_get_2 "NoCollision")
                  (Utilities|Array|Add (Variables|Default|GetFadedSegments) (LocalVariables|GetCurrentSelectedMesh))
                  (Components|StaticMesh|SetStaticMesh (LocalVariables|GetCurrentSelectedMesh) (Utilities|Struct|BreakFArrowIndicator_SegmentsConfig (Variables|Arrow|GetSegments)))
                  (bind _returnvalue_2 (Rendering|Material|CreateDynamicMaterialInstance (Utilities|Struct|BreakFArrowIndicator_SegmentsConfig (Variables|Arrow|GetSegments)) "None" "None" :!class /Script/Engine.KismetMaterialLibrary))
                  (bind _output_get_3 (LocalVariables|SetCurrentSelectedMaterial _returnvalue_2))
                  (Rendering|Material|SetMaterial (LocalVariables|GetCurrentSelectedMesh) 0 _output_get_3)))
              (else
                (bind _output_get_4 (LocalVariables|SetCurrentSelectedMesh (Utilities|Array|Get(acopy) (Variables|Default|GetFadedSegments) (LocalVariables|GetFadedSegmentIndex))))
                (bind _asmaterial_instance_dynamic (Utilities|Casting|CastToMaterialInstanceDynamic (Rendering|Material|GetMaterial _output_get_4 0)))
                (LocalVariables|SetCurrentSelectedMaterial _asmaterial_instance_dynamic)
                (Transformation|SetRelativeTransform (LocalVariables|GetCurrentSelectedMesh) (LocalVariables|GetCurrentSegmentTransform) false false)
                (Development|SetHiddeninGame (LocalVariables|GetCurrentSelectedMesh) false false)))
            (Rendering|Material|SetScalarParameterValue (LocalVariables|GetCurrentSelectedMaterial) "Opacity" (Math|Float|Lerp _minfade _maxfade (Segments|GetFadeOpacity (LocalVariables|GetCumulativeOffset) (LocalVariables|GetSplineLenght))) :!class /Script/Engine.MaterialInstanceDynamic)
            (Math|Integer|IncrementInt (LocalVariables|GetFadedSegmentIndex)
              (:%20%20
                _))
            (else
              (if (> (+ (LocalVariables|GetInstancedSegmentIndex) 1) (LocalVariables|GetCurrentInstancedCount))
                (Components|InstancedStaticMesh|AddInstance (Variables|Default|GetSegmentsMeshInstance) (LocalVariables|GetCurrentSegmentTransform) false)
                (else
                  (Components|InstancedStaticMesh|UpdateInstanceTransform (Variables|Default|GetSegmentsMeshInstance) (LocalVariables|GetInstancedSegmentIndex) (LocalVariables|GetCurrentSegmentTransform) false (not (< (+ (LocalVariables|GetCumulativeOffset) _distancebetweensegment _fadedistance) (LocalVariables|GetSplineLenght))) false)))
              (Math|Integer|IncrementInt (LocalVariables|GetInstancedSegmentIndex)
                (:%20%20
                  _))))
          (LocalVariables|SetCumulativeOffset (+ (LocalVariables|GetCumulativeOffset) (Utilities|Struct|BreakFArrowIndicator_SegmentsConfig (Variables|Arrow|GetSegments)))))
        (Clear|ClearUnusedInstancedSegments (LocalVariables|GetInstancedSegmentIndex))
        (Clear|ClearUnusedStaticSegments (LocalVariables|GetFadedSegmentIndex))
        (else
          (Clear|ClearUnusedInstancedSegments)
          (Clear|ClearUnusedStaticSegments))))))

(fn UpdateHead
  (Utilities|IsValid (Variables|Default|GetHeadMeshInstance)
    (:Is%20Valid
      (Transformation|SetRelativeTransform (Variables|Default|GetHeadMeshInstance) (Segments|GetSegmentTransform (- (- (Spline|GetSplineLength (Variables|Default|GetSpline)) (Utilities|Struct|BreakFArrowIndicator_HeadConfig (Variables|Arrow|GetHead))) 0.01) (Utilities|Struct|BreakFArrowIndicator_HeadConfig (Variables|Arrow|GetHead))) false false))))

(fn ForceUpdate
  (Update|UpdateSpline)
  (Update|UpdateSegments)
  (Update|UpdateHead))

(fn SetMaxHeight
  (params (MaxHeight :type Float%20%28double-precision%29) (bForceUpdate :type Boolean))
  (Utilities|Struct|SetmembersinFArrowIndicator_SegmentsConfig (Variables|Arrow|GetSegments) MaxHeight)
  (if bForceUpdate
    (Update|UpdateSpline)
    (Update|UpdateSegments)
    (Update|UpdateHead)))

(fn SetTransformSegment
  (params (TransformSegment :type Transform) (bForceUpdate :type Boolean))
  (Utilities|Struct|SetmembersinFArrowIndicator_SegmentsConfig (Variables|Arrow|GetSegments) TransformSegment)
  (if bForceUpdate
    (Update|UpdateSpline)
    (Update|UpdateSegments)
    (Update|UpdateHead)))

(fn SetSegmentOffset
  (params (InitialSegmentOffset :type Float%20%28double-precision%29) (FinalSegmentOffset :type Float%20%28double-precision%29) (bForceUpdate :type Boolean))
  (Utilities|Struct|SetmembersinFArrowIndicator_SegmentsConfig (Variables|Arrow|GetSegments) InitialSegmentOffset FinalSegmentOffset)
  (if bForceUpdate
    (Update|UpdateSegments)))

(fn SetIncludeHeadFinalOffset
  (params (bIncludeHeadFinalOffset :type Boolean) (bForceUpdate :type Boolean))
  (Utilities|Struct|SetmembersinFArrowIndicator_SegmentsConfig (Variables|Arrow|GetSegments) bIncludeHeadFinalOffset)
  (if bForceUpdate
    (Update|UpdateSegments)))

(fn SetSpeed
  (params (Speed :type Float%20%28double-precision%29))
  (Utilities|Struct|SetmembersinFArrowIndicator_SegmentsConfig (Variables|Arrow|GetSegments) Speed))

(fn SetFadeDistance
  (params (FadeDistance :type Float%20%28double-precision%29) (bForceUpdate :type Boolean))
  (Utilities|Struct|SetmembersinFArrowIndicator_SegmentsConfig (Variables|Arrow|GetSegments) FadeDistance)
  (if bForceUpdate
    (Update|UpdateSegments)))

(fn SetFade
  (params (InitialSegmentOffset :type Float%20%28double-precision%29) (FinalSegmentOffset :type Float%20%28double-precision%29) (bForceUpdate :type Boolean))
  (Utilities|Struct|SetmembersinFArrowIndicator_SegmentsConfig (Variables|Arrow|GetSegments) InitialSegmentOffset FinalSegmentOffset)
  (if bForceUpdate
    (Update|UpdateSegments)))

(fn SetSegmentsConfig
  (params (Config :type F%20Arrow%20Indicator%20Segments%20Config%20Structure) (bForceUpdate :type Boolean))
  (bind _output_get (Variables|Arrow|SetSegments Config))
  (Set|Segments|SetSegmentsMesh (.SegmentsMesh (Utilities|Struct|BreakFArrowIndicator_SegmentsConfig _output_get)))
  (Set|Segments|SetSegmentsMaterial (.SegmentsMaterial (Utilities|Struct|BreakFArrowIndicator_SegmentsConfig _output_get)))
  (if bForceUpdate
    (Update|UpdateSpline)
    (Update|UpdateSegments)
    (Update|UpdateHead)))

(fn SetHeadMesh
  (params (HeadMesh :type Static%20Mesh%20Object%20Reference))
  (bind _head (Variables|Arrow|GetHead))
  (bind _headmaterial (Utilities|Struct|BreakFArrowIndicator_HeadConfig _head))
  (Utilities|IsValid HeadMesh
    (:Is%20Valid
      (Utilities|Struct|SetmembersinFArrowIndicator_HeadConfig (Variables|Arrow|GetHead) HeadMesh)
      (Utilities|IsValid (Variables|Default|GetHeadMeshInstance)
        (:Is%20Valid
          (Components|StaticMesh|SetStaticMesh (Variables|Default|GetHeadMeshInstance) HeadMesh))
        (:Is%20Not%20Valid
          (bind _returnvalue (AddComponent|AddStaticMeshComponent false))
          (bind _output_get (Variables|Default|SetHeadMeshInstance _returnvalue))
          (Components|StaticMesh|SetStaticMesh _output_get (Utilities|Struct|BreakFArrowIndicator_HeadConfig (Variables|Arrow|GetHead)))
          (Collision|SetCollisionEnabled (Variables|Default|GetHeadMeshInstance) "NoCollision")
          (Utilities|IsValid _headmaterial
            (:Is%20Valid
              (bind _returnvalue_2 (Rendering|Material|CreateDynamicMaterialInstance _headmaterial "None" "None" :!class /Script/Engine.KismetMaterialLibrary))
              (Rendering|Material|SetMaterial (Variables|Default|GetHeadMeshInstance) 0 _returnvalue_2))))))))

(fn SetHeadMaterial
  (params (HeadMaterial :type Material%20Interface%20Object%20Reference))
  (Utilities|IsValid HeadMaterial
    (:Is%20Valid
      (Utilities|Struct|SetmembersinFArrowIndicator_HeadConfig (Variables|Arrow|GetHead) HeadMaterial)
      (Utilities|IsValid (Variables|Default|GetHeadMeshInstance)
        (:Is%20Valid
          (bind _returnvalue (Rendering|Material|CreateDynamicMaterialInstance HeadMaterial "None" "None" :!class /Script/Engine.KismetMaterialLibrary))
          (Rendering|Material|SetMaterial (Variables|Default|GetHeadMeshInstance) 0 _returnvalue))))))

(fn SetTransformHead
  (params (TransformHead :type Transform) (bForceUpdate :type Boolean))
  (Utilities|Struct|SetmembersinFArrowIndicator_HeadConfig (Variables|Arrow|GetHead) TransformHead)
  (if bForceUpdate
    (Update|UpdateHead)))

(fn SetHeadOffset
  (params (HeadOffset :type Float%20%28double-precision%29) (bForceUpdate :type Boolean))
  (Utilities|Struct|SetmembersinFArrowIndicator_HeadConfig (Variables|Arrow|GetHead) HeadOffset)
  (if bForceUpdate
    (Update|UpdateHead)))

(fn SetHeadConfig
  (params (Config :type F%20Arrow%20Indicator%20Head%20Config%20Structure) (bForceUpdate :type Boolean))
  (bind _output_get (Variables|Arrow|SetHead Config))
  (Set|Head|SetHeadMesh (.HeadMesh (Utilities|Struct|BreakFArrowIndicator_HeadConfig _output_get)))
  (Set|Head|SetHeadMaterial (.HeadMaterial (Utilities|Struct|BreakFArrowIndicator_HeadConfig _output_get)))
  (if bForceUpdate
    (Update|UpdateHead)))

(fn SetStart
  (params (WorldStart :type Vector))
  (bind _output_get (Variables|Arrow|SetEndPosition (- (+ (Variables|Arrow|GetEndPosition) (Transformation|GetActorLocation)) WorldStart)))
  (Transformation|SetActorLocationAndRotation WorldStart (Math|Rotator|FindLookatRotation (Math|Vector|MakeVector 0.0 0.0 0.0) (Math|Vector|MakeVector (.X (Math|Vector|BreakVector _output_get)) (.Y (Math|Vector|BreakVector _output_get)) 0.0)))
  ;[1 1 1] If deed update next tick, just update the spline point
  (if (CallFunction|NeedUpdateDuringTick)
    (Update|UpdateSpline)
    (else
      (Update|ForceUpdate))))

(fn SetEnd
  (params (WorldEnd :type Vector))
  (bind _output_get (Variables|Arrow|SetEndPosition (- WorldEnd (Transformation|GetActorLocation))))
  (Transformation|SetWorldRotation (Variables|Default|GetSpline) (Math|Rotator|FindLookatRotation (Math|Vector|MakeVector 0.0 0.0 0.0) (Math|Vector|MakeVector (.X (Math|Vector|BreakVector _output_get)) (.Y (Math|Vector|BreakVector _output_get)) 0.0)) false false)
  ;[1 1 1] If deed update next tick, just update the spline point
  (if (CallFunction|NeedUpdateDuringTick)
    (Update|UpdateSpline)
    (else
      (Update|ForceUpdate))))

(fn SetStartEnd
  (params (WorldStart :type Vector) (WorldEnd :type Vector))
  (bind _output_get (Variables|Arrow|SetEndPosition (- WorldEnd WorldStart)))
  (Transformation|SetActorLocationAndRotation WorldStart (Math|Rotator|FindLookatRotation (Math|Vector|MakeVector 0.0 0.0 0.0) (Math|Vector|MakeVector (.X (Math|Vector|BreakVector _output_get)) (.Y (Math|Vector|BreakVector _output_get)) 0.0)))
  ;[1 1 1] If deed update next tick, just update the spline point
  (if (CallFunction|NeedUpdateDuringTick)
    (Update|UpdateSpline)
    (else
      (Update|ForceUpdate))))

(fn NeedUpdateDuringTick
  (return (and (!= (Utilities|Struct|BreakFArrowIndicator_SegmentsConfig (Variables|Arrow|GetSegments)) 0.0) (Variables|Arrow|GetbUpdateEveryTick))))