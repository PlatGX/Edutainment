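; BP_GPTManager is a manager actor that steps through GPT assistant actors in sequence, handling both image-response and text-response types.
; On BeginPlay it gathers actors tagged GPTAction, inserts them by ActivateOrder, spawns a MetaHuman head far below the origin and enables input.
; Open, Send and End events act on the assistant at OpenIndex, with End advancing the index.
; A debug key also triggers opening.
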(event Custom|OpenNextGPT
  (bind _gptactorsorganized (Variables|Default|GetGPTActorsOrganized))
  (bind _openindex (Variables|Default|GetOpenIndex))
  (bind _output (Utilities|Array|Get(acopy) _gptactorsorganized _openindex))
  (bind _asbp_image_response_gptassistant (Utilities|Casting|CastToBP_ImageResponseGPTAssistant _output)
    (:then
      (Default|Activate _asbp_image_response_gptassistant))
    (:CastFailed
      (bind _asbp_response_gptassistant (Utilities|Casting|CastToBP_ResponseGPTAssistant _output))
      (Default|Activate _asbp_response_gptassistant))))

(event Custom|EndCurrentGPTWindow
  (bind _gptactorsorganized (Variables|Default|GetGPTActorsOrganized))
  (bind _openindex (Variables|Default|GetOpenIndex))
  (bind _output (Utilities|Array|Get(acopy) _gptactorsorganized _openindex))
  (bind _asbp_image_response_gptassistant (Utilities|Casting|CastToBP_ImageResponseGPTAssistant _output)
    (:then
      (Default|Deactivate _asbp_image_response_gptassistant))
    (:CastFailed
      (bind _asbp_response_gptassistant (Utilities|Casting|CastToBP_ResponseGPTAssistant _output))
      (Default|Deactivate _asbp_response_gptassistant)))
  (Math|Integer|IncrementInt (Variables|Default|GetOpenIndex)))

(event Custom|SendCurrentGPTWindow
  (bind _gptactorsorganized (Variables|Default|GetGPTActorsOrganized))
  (bind _openindex (Variables|Default|GetOpenIndex))
  (bind _output (Utilities|Array|Get(acopy) _gptactorsorganized _openindex))
  (bind _asbp_image_response_gptassistant (Utilities|Casting|CastToBP_ImageResponseGPTAssistant _output)
    (:then
      (Default|SendImage _asbp_image_response_gptassistant))
    (:CastFailed
      (bind _asbp_response_gptassistant (Utilities|Casting|CastToBP_ResponseGPTAssistant _output))
      (Default|SendMessage _asbp_response_gptassistant))))

(event EventBeginPlay
  (|Init))

(event Input|KeyboardEvents|DebugKey0
  (params (Key :type Key%20Structure :default "None") (ActionValue :type Input%20Action%20Value%20Structure))
  (:Pressed
    (CallFunction|OpenNextGPT)))

(fn ConstructionScript)