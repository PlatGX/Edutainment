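; Side-panel GPT assistant actor that takes typed text, Whisper-transcribed voice or screen captures and sends them through AIITKComponentBP.
; Replies stream into the chat widget, join the message history, then go to ElevenLabs for speech.
; An EventSelector tool offers GPT BSOD, color-change and fire effects, though RunFunctionLogic, which dispatches them, has no caller here.
; Init builds the widget, tool and material, and sets hardcoded OpenAI and ElevenLabs API keys.
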(event `CaptureScreen`
  (bind _returnvalue (`KismetSystemLibrary.GetProjectDirectory`))
  (`SceneCaptureComponent2D.CaptureScene` (`self.SceneCaptureComponent2D`))
  (`KismetSystemLibrary.Delay` 0.2)
  (`KismetRenderingLibrary.ExportRenderTarget` (`self.RT_UserScreen`) _returnvalue "UserScreen")
  (`KismetSystemLibrary.Delay` 0.2)
  (bind _returnvalue_2 (`OpenAIFunctionLibrary.LoadTextureFromDisk` (`KismetStringLibrary.Concat_StrStr` _returnvalue "UserScreen")))
  (set `self.CurrentScreen` _returnvalue_2)
  (`self.Send Screen`))

(event `ToggleRecording`
  (bind _aiitkcomponentbp (`self.AIITKComponentBP`))
  ;[0 0 0] Capture voice
  (`/Engine/EditorBlueprintResources/StandardMacros.FlipFlop`
    (:`A`
      (`/AIIntegrationToolkit/Core/Components/AIITKComponentBP.StartAudioCapture` _aiitkcomponentbp))
    (:`B`
      (`/AIIntegrationToolkit/Core/Components/AIITKComponentBP.StopAudioCaptureAndSave` _aiitkcomponentbp "TempVoice"))))

(event `self.ReceiveBeginPlay`
  (bind (_location _rotation) (`Controller.GetPlayerViewPoint` (`GameplayStatics.GetPlayerController` 0)))
  ;[0 0 0] Init
  (`KismetSystemLibrary.Delay` 0.2)
  (`|ExecutionSequence`
    (:`then_0`
      (bind _returnvalue (`|CreateWidget` "/Game/GPT/W_SideGPTAssistant.W_SideGPTAssistant_C"))
      (`UserWidget.AddToViewport` _returnvalue 0)
      (bind _output_get (set `self.ChatInterfaceWidgetRef` _returnvalue))
      (set `/Game/GPT/W_SideGPTAssistant.ShowSystemMessages` (`self.ShowSystemMessages`) _output_get))
    (:`then_1`
      (`self.ConstructSelectorFunction`))
    (:`then_2`
      (`self.ConstructDynamicMaterial`))
    (:`then_3`
      (`AIITKDeveloperSettings.SetAPIKey` "OpenAI" "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")
      (`AIITKDeveloperSettings.SetAPIKey` "Labs11" "sk_e229d49041bf466d481f1e59f903dd901892e99e82f3e679"))
    (:`then_4`
      (`KismetSystemLibrary.Delay` 0.2)
      (`SceneComponent.K2_SetWorldTransform` (`self.SceneCaptureComponent2D`) (`KismetMathLibrary.MakeTransform` _location _rotation) false false)
      (bind _returnvalue_2 (`GameplayStatics.GetActorOfClass` "/Script/Engine.PostProcessVolume"))
      (set `SceneCaptureComponent2D.PostProcessSettings` (`PostProcessVolume.Settings` _returnvalue_2) (`self.SceneCaptureComponent2D`)))
    (:`then_5`
      (`KismetSystemLibrary.Delay` 0.2)
      (bind _returnvalue_3 (`GameplayStatics.GetActorOfClass` "/Game/GPT/BP_MetahumanHead.BP_MetahumanHead_C"))
      (set `self.BP_MetahumanHead` _returnvalue_3))))

(event `Send Message`
  (bind _gptparams (`self.GPTParams`))
  ;[0 0 0] Request W/ Text
  (`self.AddUserMessage`)
  (`/Game/Blueprints/GI_Dynamics.UpdateTranscript` (cast `/Game/Blueprints/GI_Dynamics` (`GameplayStatics.GetGameInstance`) :!pure true) _gptparams)
  (`/AIIntegrationToolkit/Core/Components/AIITKComponentBP.SendRequestToGPT` (`self.AIITKComponentBP`) _gptparams))

(event `self.AIITKComponentBP.OnAudioCaptureSaved`
  (params (WAVFilePath :type String))
  ;[0 0 0] Whisper request
  (bind _structout (setmembers `WhisperAPIParams` :`StructRef` (`self.WhisperParams`) :`FilePath` WAVFilePath))
  (`/AIIntegrationToolkit/Core/Components/AIITKComponentBP.SendRequestToWhisper` (`self.AIITKComponentBP`) _structout))

(event `Send Screen`
  ;[0 0 0] Request W/ Image
  (`self.AddUserScreen`)
  (`/AIIntegrationToolkit/Core/Components/AIITKComponentBP.SendRequestToGPT` (`self.AIITKComponentBP`) (`self.GPTParams`)))

(event `self.AIITKComponentBP.OnWhisperTranscriptGenerated`
  (params (Transcription :type String))
  ;[0 0 0] Whisper response
  (`self.Send Message From Voice` Transcription))

(event `Send Message From Voice`
  (params (`User Message` :type String))
  (bind _gptparams (`self.GPTParams`))
  (`self.AddUserSTTMessage` `User Message`)
  (`/Game/Blueprints/GI_Dynamics.UpdateTranscript` (cast `/Game/Blueprints/GI_Dynamics` (`GameplayStatics.GetGameInstance`) :!pure true) _gptparams)
  (`/AIIntegrationToolkit/Core/Components/AIITKComponentBP.SendRequestToGPT` (`self.AIITKComponentBP`) _gptparams))

(event `self.AIITKComponentBP.OnGPTChunkReceived`
  (params (Completion :type "GPTChatCompletion Structure"))
  ;[0 0 0] Responses
  (bind _responsecontent (`self.GetFirstChoiceContent` Completion))
  (`/Game/GPT/W_SideGPTAssistant.UpdateLastMessageOnScreen` (`self.ChatInterfaceWidgetRef`) _responsecontent))

(event `self.AIITKComponentBP.OnGPTCompleted`
  (params (Completion :type "GPTChatCompletion Structure"))
  ;[0 0 0] Responses
  (bind _output_get (set `self.CurrentChatCompletion` Completion))
  (`self.AddResponseMessage` _output_get)
  (bind _structout (setmembers `11LabsRequestParams` :`StructRef` (`self.11LabsRequest`) :`TextPrompt` (`OpenAIFunctionLibrary.GetMessageContent` (`OpenAIFunctionLibrary.GetResponseMessage` _output_get))))
  (bind _11labsinstance (`/AIIntegrationToolkit/Core/Components/AIITKComponentBP.SendRequestTo11Labs` (`self.AIITKComponentBP`) _structout))
  (add `TextToSpeechAPI.OnAudioWithAlignmentGenerated` _11labsinstance (`|CreateDelegate` :!event `AudioGenerated`))
  (add `TextToSpeechAPI.OnProceduralAudioFinished` _11labsinstance (`|CreateDelegate` :!event `StopCurrentSound`)))

(fn `AddResponseMessage`
  (params (ChatCompletion :type "GPTChatCompletion Structure (by ref)"))
  (bind _gptparams (`self.GPTParams`))
  (`KismetArrayLibrary.Array_Add` (`.Messages` (break `GPTChatPromptParams` (`self.GPTParams`))) (`OpenAIFunctionLibrary.GetResponseMessage` ChatCompletion))
  (`/Game/GPT/W_SideGPTAssistant.UpdateMessagesOnScreen` (`self.ChatInterfaceWidgetRef`) _gptparams)
  (`/AIIntegrationToolkit/Core/Components/AIITKComponentBP.TruncateMessages` (`self.AIITKComponentBP`) _gptparams))

(fn `AddSystemMessage`
  (params (Content :type String))
  (`KismetArrayLibrary.Array_Add` (`.Messages` (break `GPTChatPromptParams` (`self.GPTParams`))) (make `GPTChatMessage` "system" "" (make `SystemMessage` "system" Content) (struct :`Role` "user") (make `AssistantMessage` ""))))

(fn `AddToolResponseMessage`
  (params (`Tool Message` :type "ToolMessage Structure"))
  (bind (_role _content _toolcallid) (break `ToolMessage` `Tool Message`))
  (`KismetArrayLibrary.Array_Add` (`.Messages` (break `GPTChatPromptParams` (`self.GPTParams`))) (make `GPTChatMessage` :`Role` "tool" :`ToolMessage` (make `ToolMessage` _content _toolcallid))))

(fn `AddUserMessage`
  (bind _chatinterfacewidgetref (`self.ChatInterfaceWidgetRef`))
  (`KismetArrayLibrary.Array_Add` (`.Messages` (break `GPTChatPromptParams` (`self.GPTParams`))) (make `GPTChatMessage` :`Role` "user" :`UserMessage` (make `UserMessage` (`|MakeArray` (make `ContentPart` "Text" (`KismetTextLibrary.Conv_TextToString` (`MultiLineEditableText.GetText` (`/Game/GPT/W_SideGPTAssistant.UserPrompt` (`self.ChatInterfaceWidgetRef`))))) :!type "ContentPart Structure"))))
  (`/Game/GPT/W_SideGPTAssistant.UpdateMessagesOnScreen` _chatinterfacewidgetref (`self.GPTParams`))
  (`/Game/GPT/W_SideGPTAssistant.ClearUserPrompt` _chatinterfacewidgetref)
  (`/Game/GPT/W_SideGPTAssistant.AddNewChatObject` (`self.ChatInterfaceWidgetRef`) (make `GPTChatMessage` "assistant")))

(fn `AddUserScreen`
  (bind _returnvalue (`OpenAIFunctionLibrary.TextureToBase64` (`self.CurrentScreen`)))
  (`KismetArrayLibrary.Array_Add` (`.Messages` (break `GPTChatPromptParams` (`self.GPTParams`))) (make `GPTChatMessage` :`Role` "user" :`UserMessage` (make `UserMessage` (`|MakeArray` (make `ContentPart` "Image" _returnvalue) :!type "ContentPart Structure"))))
  (`/Game/GPT/W_SideGPTAssistant.AddNewChatObject` (`self.ChatInterfaceWidgetRef`) (make `GPTChatMessage` "assistant")))

(fn `AddUserSTTMessage`
  (params (`User Message` :type String))
  (`KismetArrayLibrary.Array_Add` (`.Messages` (break `GPTChatPromptParams` (`self.GPTParams`))) (make `GPTChatMessage` :`Role` "user" :`UserMessage` (make `UserMessage` (`|MakeArray` (make `ContentPart` "Text" `User Message`) :!type "ContentPart Structure"))))
  (`/Game/GPT/W_SideGPTAssistant.UpdateMessagesOnScreen` (`self.ChatInterfaceWidgetRef`) (`self.GPTParams`))
  (`/Game/GPT/W_SideGPTAssistant.AddNewChatObject` (`self.ChatInterfaceWidgetRef`) (make `GPTChatMessage` "assistant")))

(fn `AudioGenerated`
  (params (GeneratedAudio :type "SoundWave Object Reference") (AlignmentData :type "CharacterAlignment Structure (by ref)"))
  (bind _speaker (`self.Speaker`))
  (if (`AudioComponent.IsPlaying` (`self.Speaker`))
    (`self.StopCurrentSound`))
  (`AudioComponent.SetSound` _speaker GeneratedAudio)
  (`AudioComponent.Play` _speaker 0.0)
  (`KismetSystemLibrary.PrintString` "PLAYING TTS")
  (return))

(fn `StopCurrentSound`
  (`AudioComponent.Stop` (`self.Speaker`))
  (return))

(fn `UserConstructionScript`)