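; BP_Tire is a prototype tire that rolls along its spline in a repeating, accelerating loop.
; Each tick, Speed advances a distance value that positions the static mesh on the spline in local space and drives its roll, with yaw fixed.
; Acceleration is added per frame without delta-time scaling.
; Reaching the chosen spline point resets distance and speed, while hitting the speed cap resets only speed.
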(event `self.ReceiveTick`
  (params (DeltaSeconds :type "Float (single-precision)"))
  (bind _output_get (set `self.Delta` (+ (* DeltaSeconds (`self.Speed`)) (`self.Delta`))))
  (`SceneComponent.K2_SetRelativeLocationAndRotation` (`self.StaticMesh`) (`SplineComponent.GetLocationAtDistanceAlongSpline` (`self.Spline`) _output_get "Local") (`KismetMathLibrary.MakeRotator` (* (`self.Delta`) (`self.AngularSpeed`) 1.0) 0.0 90.0) false false)
  (set `self.Speed` (+ (`self.Acceleration`) (`self.Speed`)))
  (if (>= (`self.Delta`) (`SplineComponent.GetDistanceAlongSplineAtSplinePoint` (`self.Spline`) (`self.PointIndex`)))
    (set `self.Delta` 0.0)
    (set `self.Speed` 500.0 :!label _label)
    (elif (>= (`self.Speed`) 3000.0)
      (goto _label))))

(fn `UserConstructionScript`)