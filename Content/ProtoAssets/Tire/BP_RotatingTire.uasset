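; BP_RotatingTire is a tire prop that spins its static mesh with a steadily increasing speed.
; Each Tick sets relative roll to accumulated time times AngularSpeed at a fixed yaw, resetting the time once the angle nears a full turn.
; AngularSpeed grows by AngularAceleration every frame, independent of delta time, and drops to a lower speed after passing an upper limit, so the spin-up repeats.
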(event `self.ReceiveTick`
  (params (DeltaSeconds :type "Float (single-precision)"))
  (set `self.Delta` (+ DeltaSeconds (`self.Delta`)))
  (`SceneComponent.K2_SetRelativeRotation` (`self.StaticMesh`) (`KismetMathLibrary.MakeRotator` (* (`self.Delta`) (`self.AngularSpeed`) 1.0) 0.0 90.0) false false)
  (set `self.AngularSpeed` (+ (`self.AngularAceleration`) (`self.AngularSpeed`)))
  (if (> (* (`self.Delta`) (`self.AngularSpeed`) 1.0) 359.0)
    (set `self.Delta` 0.0))
  (if (> (`self.AngularSpeed`) 2500.0)
    (set `self.AngularSpeed` 500.0)))

(fn `UserConstructionScript`)