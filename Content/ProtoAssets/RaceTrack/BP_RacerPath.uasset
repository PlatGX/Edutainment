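; BP_RacerPath drives a TrainFront actor along the spline of a referenced Path, starting at BeginPlay.
; A timeline supplies an alpha that maps to distance along the spline plus CarOffset, setting world location and rotation each update.
; The timeline's Speed track feeds back into its play rate to vary pace.
; CalculateDistance sets CarOffset to the TrainFront–TrainCar distance, but nothing in this graph calls it.
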(event `self.ReceiveBeginPlay`
  (`self.StartTimeline`))

(event `StartTimeline`
  (bind _path (`/Game/RollerCoasterAnim/BP_Path.Path` (`self.Path`)))
  (bind (_direction _pointonpath _speed) (`Timeline|T_Path`)
    (:`Update`
      (`TimelineComponent.SetPlayRate` (`self.T_Path`) _speed)
      (bind _returnvalue (+ (`KismetMathLibrary.Lerp` 0.0 (`SplineComponent.GetSplineLength` _path) _pointonpath) (`self.CarOffset`)))
      (`self.K2_SetActorLocationAndRotation` (`self.TrainFront`) (`SplineComponent.GetLocationAtDistanceAlongSpline` _path _returnvalue "World") (`SplineComponent.GetRotationAtDistanceAlongSpline` _path _returnvalue "World") false false))))

(event `CalculateDistance`
  (bind (_returnvalue_x _returnvalue_y _returnvalue_z) (`KismetMathLibrary.BreakVector` (`SceneComponent.K2_GetComponentLocation` (`Actor.RootComponent` (`self.TrainFront`)))))
  (bind (_returnvalue_x_2 _returnvalue_y_2 _returnvalue_z_2) (`KismetMathLibrary.BreakVector` (`SceneComponent.K2_GetComponentLocation` (`Actor.RootComponent` (`self.TrainCar`)))))
  (set `self.CarOffset` (`KismetMathLibrary.Sqrt` (+ (`KismetMathLibrary.Square` (- _returnvalue_x _returnvalue_x_2)) (`KismetMathLibrary.Square` (- _returnvalue_y _returnvalue_y_2)) (`KismetMathLibrary.Square` (- _returnvalue_z _returnvalue_z_2))))))

(fn `UserConstructionScript`)