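; Merry-go-round prototype actor that spins continuously around its vertical axis once play begins.
; A Rotate event accumulates frame delta time scaled by Speed into DeltaT and applies it as the actor's absolute yaw.
; The event re-calls itself after a zero-length Delay, forming a per-frame loop in place of Event Tick.
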(event `self.ReceiveBeginPlay`
  (`self.Rotate`))

(event `Rotate`
  (bind _output_get (set `self.DeltaT` (+ (`self.DeltaT`) (* (`GameplayStatics.GetWorldDeltaSeconds`) (`self.Speed`)))))
  (`self.K2_SetActorRotation` (`KismetMathLibrary.MakeRotator` 0.0 0.0 _output_get))
  (`KismetSystemLibrary.Delay` 0.0)
  (`self.Rotate`))

(fn `UserConstructionScript`)