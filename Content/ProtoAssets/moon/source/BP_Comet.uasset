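; BP_Comet is an actor that repeatedly flies its component named Earth along a spline path, starting at BeginPlay.
; Launch adds frame time to Delta, divides it by Period, and places the component at that spline time in world space.
; It re-triggers itself through a zero-length Delay instead of Tick until the path completes, then resets Delta and waits Offset seconds before the next pass.
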(event `self.ReceiveBeginPlay`
  (`self.Launch`))

(event `Launch`
  (bind _returnvalue (/ (+ (`self.Delta`) (`GameplayStatics.GetWorldDeltaSeconds`)) (`self.Period`)))
  (set `self.Delta` (+ (`self.Delta`) (`GameplayStatics.GetWorldDeltaSeconds`)))
  (`SceneComponent.K2_SetWorldLocation` (`self.Earth`) (`SplineComponent.GetLocationAtTime` (`self.Spline`) _returnvalue "World" false) false false)
  (if (<= _returnvalue 1.0)
    (`KismetSystemLibrary.Delay` 0.0)
    (`self.Launch`)
    (else
      (set `self.Delta` 0.0)
      (`KismetSystemLibrary.Delay` (`self.Offset`))
      (`self.Launch`))))

(fn `UserConstructionScript`)