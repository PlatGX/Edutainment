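; BP_GearOpt is a gear prop that spins continuously around its yaw axis.
; The construction script and BeginPlay both apply the GearOpt mesh to the Gear component.
; A Rotate event accumulates a yaw angle from frame delta time, Speed and a Clockwise sign, then sets the relative rotation.
; It re-calls itself after a zero-length Delay, looping each frame without Event Tick.
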(event `self.ReceiveBeginPlay`
  (`StaticMeshComponent.SetStaticMesh` (`self.Gear`) (`self.GearOpt`))
  (`self.Rotate`))

(event `Rotate`
  (bind _output_get (set `self.Delta` (+ (* (`GameplayStatics.GetWorldDeltaSeconds`) (`self.Speed`) (`KismetMathLibrary.SelectFloat` 1.0 -1.0 (`self.Clockwise? `))) (`self.Delta`))))
  (`SceneComponent.K2_SetRelativeRotation` (`self.Gear`) (`KismetMathLibrary.MakeRotator` 0.0 0.0 _output_get) false false)
  (`KismetSystemLibrary.Delay` 0.0)
  (`self.Rotate`))

(fn `UserConstructionScript`
  (`StaticMeshComponent.SetStaticMesh` (`self.Gear`) (`self.GearOpt`)))