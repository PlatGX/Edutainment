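; BP_Arrow is a conveyor prototype actor that endlessly slides its arrow component along local X as a repeating animation.
; From BeginPlay, MoveArrow accumulates frame time and lerps the relative X position from zero toward a fixed negative offset over Period seconds, then restarts the timer.
; The event re-calls itself through a zero-length Delay, giving a per-frame loop without using Event Tick.
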(event `self.ReceiveBeginPlay`
  (`self.MoveArrow`))

(event `MoveArrow`
  (bind _output_get (set `self.DeltaTime` (+ (`self.DeltaTime`) (`GameplayStatics.GetWorldDeltaSeconds`))))
  (if (<= _output_get (`self.Period`))
    (`SceneComponent.K2_SetRelativeLocation` (`self.arrow-basic`) (`KismetMathLibrary.MakeVector` (`KismetMathLibrary.Lerp` 0.0 -200.0 (`KismetMathLibrary.FClamp` (/ (`self.DeltaTime`) (`self.Period`))))) false false)
    (`KismetSystemLibrary.Delay` 0.0)
    (`self.MoveArrow`)
    (else
      (set `self.DeltaTime` 0.0)
      (`KismetSystemLibrary.Delay` 0.0)
      (`self.MoveArrow`))))

(fn `UserConstructionScript`)